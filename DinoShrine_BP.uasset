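; Placeable ARK dino shrine structure that spawns a configurable creature at an offset and respawns it after a delay when it dies.
; On server BeginPlay it loads settings, spawns the dino, optionally applies a visual buff and binds its death.
; Settings persist in the DinoShrine SaveGame slot by structure ID; saving triggers another spawn.
; A multi-use entry spawns ShrineCommActor for the settings UI, with debug entries in non-shipping builds.
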(event Custom|PrimalCharacterDied__DelegateSignature_Event
  (params (DiedCharacter :type Primal%20Character%20Object%20Reference))
  (bind _self self)
  (bind _persistantsettings2 (Variables|Default|GetPersistantSettings2))
  (bind _persistantsettings2_2 (Variables|Default|GetPersistantSettings2))
  (bind (_structureid _dinospawnclass _spawnbuffclass _respawndelay _spawnxoffset _spawnyoffset _spawnzoffset) (Utilities|Struct|BreakDinoShrineData _persistantsettings2))
  (bind (_structureid_2 _dinospawnclass_2 _spawnbuffclass_2 _respawndelay_2 _spawnxoffset_2 _spawnyoffset_2 _spawnzoffset_2 _bshowvisualeffect) (Utilities|Struct|BreakDinoShrineData _persistantsettings2_2))
  (bind _returnvalue (Transformation|GetActorTransform _self))
  (bind (_location _rotation _scale) (Math|Transform|BreakTransform _returnvalue))
  (bind (_x _y _z) (Math|Vector|BreakVector _location))
  ;[1 1 1] Apply settings
  (Utilities|FlowControl|RetriggerableDelay (.RespawnDelay (Utilities|Struct|BreakDinoShrineData (Variables|Default|GetPersistantSettings2))))
  (bind _returnvalue_2 (Game|SpawnActorfromClass (.DinoSpawnClass (Utilities|Struct|BreakDinoShrineData (Variables|Default|GetPersistantSettings2))) (Math|Transform|MakeTransform (Math|Vector|MakeVector (+ _x _spawnxoffset) (+ _y _spawnyoffset) (+ _z _spawnzoffset)) _rotation _scale) true))
  (bind _asprimaldinocharacter (Utilities|Casting|CastToPrimalDinoCharacter _returnvalue_2))
  (EventDispatchers|BindEventtoOnDied _asprimaldinocharacter (delegate Custom|PrimalCharacterDied__DelegateSignature_Event))
  ;;[1 1 1] Gate visual effect from config option
  (if _bshowvisualeffect
    (Class|PrimalBuff|StaticAddBuff _spawnbuffclass_2 _asprimaldinocharacter 0 0 false)))

(event Custom|ReinitShrine
  (bind _self self)
  (bind _persistantsettings2 (Variables|Default|GetPersistantSettings2))
  (bind _persistantsettings2_2 (Variables|Default|GetPersistantSettings2))
  (bind (_structureid _dinospawnclass _spawnbuffclass _respawndelay _spawnxoffset _spawnyoffset _spawnzoffset) (Utilities|Struct|BreakDinoShrineData _persistantsettings2))
  (bind (_structureid_2 _dinospawnclass_2 _spawnbuffclass_2 _respawndelay_2 _spawnxoffset_2 _spawnyoffset_2 _spawnzoffset_2 _bshowvisualeffect) (Utilities|Struct|BreakDinoShrineData _persistantsettings2_2))
  (bind _returnvalue (Transformation|GetActorTransform _self))
  (bind (_location _rotation _scale) (Math|Transform|BreakTransform _returnvalue))
  (bind (_x _y _z) (Math|Vector|BreakVector _location))
  ;[1 1 1] Apply settings
  (bind _returnvalue_2 (Game|SpawnActorfromClass (.DinoSpawnClass (Utilities|Struct|BreakDinoShrineData (Variables|Default|GetPersistantSettings2))) (Math|Transform|MakeTransform (Math|Vector|MakeVector (+ _x _spawnxoffset) (+ _y _spawnyoffset) (+ _z _spawnzoffset)) _rotation _scale) true))
  (bind _asprimaldinocharacter (Utilities|Casting|CastToPrimalDinoCharacter _returnvalue_2))
  (EventDispatchers|BindEventtoOnDied _asprimaldinocharacter (delegate Custom|PrimalCharacterDied__DelegateSignature_Event))
  ;;[1 1 1] Gate visual effect from config option
  (if _bshowvisualeffect
    (Class|PrimalBuff|StaticAddBuff _spawnbuffclass_2 _asprimaldinocharacter 0 0 false)))

(event EventBeginPlay
  (bind _self self)
  (bind _persistantsettings2 (Variables|Default|GetPersistantSettings2))
  (bind _persistantsettings2_2 (Variables|Default|GetPersistantSettings2))
  (bind (_structureid _dinospawnclass _spawnbuffclass _respawndelay _spawnxoffset _spawnyoffset _spawnzoffset) (Utilities|Struct|BreakDinoShrineData _persistantsettings2))
  (bind (_structureid_2 _dinospawnclass_2 _spawnbuffclass_2 _respawndelay_2 _spawnxoffset_2 _spawnyoffset_2 _spawnzoffset_2 _bshowvisualeffect) (Utilities|Struct|BreakDinoShrineData _persistantsettings2_2))
  (bind _returnvalue (Transformation|GetActorTransform _self))
  (bind (_location _rotation _scale) (Math|Transform|BreakTransform _returnvalue))
  (bind (_x _y _z) (Math|Vector|BreakVector _location))
  (|CallParentFunction)
  (Utilities|FlowControl|RetriggerableDelay 0.2)
  (if (not (Variables|Default|GetbIsPreviewStructure))
    (Utilities|SwitchNetAuthority
      (:DedicatedServer
        _)
      (:PlayerServer
        _))
    (Utilities|FlowControl|Sequence
      (:then_0
        (CallFunction|LoadShrineSettings))
      (:then_1
        ;[1 1 1] Apply settings
        (bind _returnvalue_2 (Game|SpawnActorfromClass (.DinoSpawnClass (Utilities|Struct|BreakDinoShrineData (Variables|Default|GetPersistantSettings2))) (Math|Transform|MakeTransform (Math|Vector|MakeVector (+ _x _spawnxoffset) (+ _y _spawnyoffset) (+ _z _spawnzoffset)) _rotation _scale) true))
        (bind _asprimaldinocharacter (Utilities|Casting|CastToPrimalDinoCharacter _returnvalue_2))
        (EventDispatchers|BindEventtoOnDied _asprimaldinocharacter (delegate Custom|PrimalCharacterDied__DelegateSignature_Event))
        ;;[1 1 1] Gate visual effect from config option
        (if _bshowvisualeffect
          (Class|PrimalBuff|StaticAddBuff _spawnbuffclass_2 _asprimaldinocharacter 0 0 false))))))

(event EventSetNewSpawnableDino
  (params (NewSpawnCreature :type Primal%20Dino%20Character%20Class%20Reference))
  ;[1 1 1] Settings from UI
  (bind _returnvalue (Class|PrimalStructure|BPGetStructureID self))
  (Variables|Default|SetPersistantSettings2 (Utilities|Struct|MakeDinoShrineData _returnvalue NewSpawnCreature "/Game/PrimalEarth/CoreBlueprints/Buffs/Buff_Liopleurodon_Magic.Buff_Liopleurodon_Magic_C" 1e+01 1e+02 1e+02 0.0 true))
  (CallFunction|SaveShrineSettings))

(fn ConstructionScript
  (|CallParentFunction))

(fn BPGetMultiUseEntries
  (params (ForPC :type Player%20Controller%20Object%20Reference) (MultiUseEntries :type Array%20of%20Multi%20Use%20Entry%20Structures))
  (bind _color (Math|Color|MakeColor 244 66 164 255))
  (LocalVariables|SetMU_Buffer MultiUseEntries)
  (Utilities|Array|Add (LocalVariables|GetMU_Buffer) (Utilities|Struct|MakeMultiUseEntry 0 "Change Dino Settings" 15679 0 false false false false false false false false false true false false false 0 "(B=175,G=175,R=175,A=255)" (Math|Color|MakeColor 66 140 244 255)))
  (if (Class|VictoryCore|IsShipping)
    _
    (else
      ;[1 1 1] Debug Options
      (Utilities|Array|AppendArray (LocalVariables|GetMU_Buffer) (Utilities|Array|MakeArray (Utilities|Struct|MakeMultiUseEntry 0 "Debug 1" 15676 0 false false false false false false false false false true false false false 0 "(B=175,G=175,R=175,A=255)" _color) (Utilities|Struct|MakeMultiUseEntry 0 "Debug 2" 15677 0 false false false false false false false false false true false false false 0 "(B=175,G=175,R=175,A=255)" _color) (Utilities|Struct|MakeMultiUseEntry 0 "Debug 3" 15678 0 false false false false false false false false false true false false false 0 "(B=175,G=175,R=175,A=255)" _color)))))
  (return (LocalVariables|GetMU_Buffer)))

(fn LoadShrineSettings
  ;[0.1091 0.9618 1] Settings retrieval
  (bind _returnvalue (Class|PrimalStructure|BPGetStructureID self))
  (CallFunction|GetShrineSave)
  (bind _shrinedata (CallFunction|GetShrineData 0 _returnvalue :!label _label))
  (if (== _returnvalue 0)
    (Variables|Default|SetPersistantSettings _shrinedata)
    (else
      (CallFunction|CreateNewShrineData 0 _returnvalue)
      (SaveGame|SaveGametoSlot 0 "DinoShrine")
      (goto _label))))

(fn SaveShrineSettings
  (CallFunction|GetShrineSave)
  (bind _returnvalue (Class|PrimalStructure|BPGetStructureID self))
  (CallFunction|ChangeShrineData 0 _returnvalue (Variables|Default|GetPersistantSettings))
  (SaveGame|SaveGametoSlot 0 "DinoShrine")
  (CallFunction|ReinitShrine))

(fn GetShrineSave
  (bind _returnvalue (SaveGame|DoesSaveGameExist "DinoShrine"))
  (if _returnvalue
    _
    (else
      (bind _returnvalue_2 (SaveGame|CreateSaveGameObject "/Game/Mods/MyMods/SpawnPillar/DinoShrineSave.DinoShrineSave_C"))
      (SaveGame|SaveGametoSlot _returnvalue_2 "DinoShrine")))
  (bind _returnvalue_3 (SaveGame|LoadGamefromSlot "DinoShrine"))
  (Utilities|Casting|CastTo _returnvalue_3)
  (return 0))

(fn BPTryMultiUse
  (params (ForPC :type Player%20Controller%20Object%20Reference) (UseIndex :type Integer))
  (Class|PrimalStructure|BPGetStructureID self)
  (switch int UseIndex
    (:15676
      ;[1 1 1] Debug options
      (Variables|Default|SetPersistantSettings "")
      (CallFunction|SaveShrineSettings :!label _label))
    (:15677
      (Variables|Default|SetPersistantSettings "")
      (goto _label))
    (:15678
      (Variables|Default|SetPersistantSettings "")
      (goto _label))
    (:15679
      (CallFunction|StartUI ForPC)))
  (return false))

(fn StartUI
  (params (For%20PC :type Player%20Controller%20Object%20Reference))
  (bind _returnvalue (Pawn|GetControlledPawn For%20PC))
  (Utilities|IsValid _returnvalue
    (:Is%20Valid
      (bind _returnvalue_2 (Game|SpawnActorfromClass "/Game/Mods/MyMods/SpawnPillar/ShrineCommActor.ShrineCommActor_C" (Transformation|GetActorTransform _returnvalue) true self (Utilities|Array|MakeArray "/Game/PrimalEarth/Dinos/Achatina/Achatina_Character_BP.Achatina_Character_BP_C" "/Game/PrimalEarth/Dinos/Ankylo/Ankylo_Character_BP.Ankylo_Character_BP_C" "/Game/PrimalEarth/Dinos/Dimorphodon/Dimorph_Character_BP.Dimorph_Character_BP_C" "/Game/PrimalEarth/Dinos/Dodo/Dodo_Character_BP.Dodo_Character_BP_C" "/Game/PrimalEarth/Dinos/DungBeetle/DungBeetle_Character_BP.DungBeetle_Character_BP_C") _returnvalue))
      (Actor|SetOwner _returnvalue_2 _returnvalue)
      (Default|Init _returnvalue_2))))